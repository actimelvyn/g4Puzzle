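; BP_Door_Actor is a locked door that swings open on overlap once its key has been found.
; At BeginPlay it binds to KeyActor's KeyFound dispatcher, which sets CanOpen.
; Entering the Box trigger with CanOpen set plays a Timeline that lerps the Hinge yaw open, and leaving it reverses the Timeline.
; The trigger does not filter which actor overlaps it.
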(event `openDoor`
  ; Door Animation
  (bind (_direction _open_door) (`Timeline|Timeline_Door` :!label _label)
    (:`Update`
      (`SceneComponent.K2_SetRelativeRotation` (`self.Hinge`) (`KismetMathLibrary.MakeRotator` 0.0 0.0 (`KismetMathLibrary.Lerp` 0.0 90.0 _open_door)) false false))))

(event `CloseDoor`
  (goto _label :!via `Reverse`))

(event `self.ReceiveBeginPlay`
  (add `/Game/keys/Main_Key_Actor.KeyFound` (`self.KeyActor`) (delegate `KeyFound`)))

(event `KeyFound`
  (set `self.canOpen` true))

(event `self.Box.OnComponentBeginOverlap`
  (params (OverlappedComponent :type "PrimitiveComponent Object Reference") (OtherActor :type "Actor Object Reference") (OtherComp :type "PrimitiveComponent Object Reference") (OtherBodyIndex :type Integer) (bFromSweep :type Boolean) (SweepResult :type "HitResult Structure (by ref)"))
  (if (`self.canOpen`)
    (`self.openDoor`)))

(event `self.Box.OnComponentEndOverlap`
  (params (OverlappedComponent :type "PrimitiveComponent Object Reference") (OtherActor :type "Actor Object Reference") (OtherComp :type "PrimitiveComponent Object Reference") (OtherBodyIndex :type Integer))
  (`self.CloseDoor`))

(fn `UserConstructionScript`)